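; BP_ObonBackup is a player character Blueprint, apparently a backup of the main character, with movement, jump and dodge driven by Enhanced Input actions.
; Keyboard left/right input is rotated by actor rotation into movement input, and the jump action starts and stops jumping.
; Dodge temporarily boosts max walk speed, using delays to restore it and gate a cooldown, printing a message while unavailable.
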(event Input|EnhancedActionEvents|EnhancedInputActionIA_KeyboardLR
  (params (ActionValue :type Vector%202D%20Structure) (ElapsedSeconds :type Float%20%28double-precision%29) (TriggeredSeconds :type Float%20%28double-precision%29) (InputAction :type Input%20Action%20Object%20Reference :default "/Game/Inputs/Actions/IA_KeyboardLR.IA_KeyboardLR"))
  ;[0 0 0] IA Keyboard Left/Right
  (Pawn|Input|AddMovementInput (Math|Vector|RotateVector (Math|Conversions|ToVector(Vector2D) ActionValue) (Transformation|GetActorRotation)) 1.0 false))

(event Input|EnhancedActionEvents|EnhancedInputActionIA_Jump
  (params (ActionValue :type Boolean) (ElapsedSeconds :type Float%20%28double-precision%29) (TriggeredSeconds :type Float%20%28double-precision%29) (InputAction :type Input%20Action%20Object%20Reference :default "/Game/Inputs/Actions/IA_Jump.IA_Jump"))
  ;[0 0 0] IA Jump
  (:Started
    (Character|Jump :!label _label))
  (:Ongoing
    (goto _label))
  (:Completed
    (Character|StopJumping)))

(event Input|EnhancedActionEvents|EnhancedInputActionIA_Dodge
  (params (ActionValue :type Boolean) (ElapsedSeconds :type Float%20%28double-precision%29) (TriggeredSeconds :type Float%20%28double-precision%29) (InputAction :type Input%20Action%20Object%20Reference :default "/Game/Inputs/Actions/IA_Dodge.IA_Dodge"))
  (bind _dodgeduration (Variables|Default|GetDodgeDuration))
  (bind _charactermovement (Variables|Character|GetCharacterMovement))
  ;[0 0 0] IA Dodge (Have to implement MAX Move Speed First!)
  (if (Variables|Default|GetIsDodgeUp)
    (Variables|Default|SetIsDodgeUp false)
    (Variables|Default|SetBaseMovementSpeed (Variables|/Script/Engine.CharacterMovementComponent|GetMaxWalkSpeed (Variables|Character|GetCharacterMovement)))
    (Variables|/Script/Engine.CharacterMovementComponent|SetMaxWalkSpeed _charactermovement (+ (Variables|/Script/Engine.CharacterMovementComponent|GetMaxWalkSpeed (Variables|Character|GetCharacterMovement)) 4e+03))
    (Utilities|FlowControl|Delay _dodgeduration)
    (Variables|/Script/Engine.CharacterMovementComponent|SetMaxWalkSpeed _charactermovement (Variables|Default|GetBaseMovementSpeed))
    (Utilities|FlowControl|Delay (- (Variables|Default|GetDodgeCooldown) _dodgeduration))
    (Variables|Default|SetIsDodgeUp true)
    (else
      (Development|PrintString "Dodge is on Cooldown" true true "(R=1.000000,G=0.000000,B=0.024480,A=1.000000)"))))

(fn ConstructionScript)