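; Player character Blueprint, apparently a backup of Nobo, that spawns Tier 0 swords overhead on a timer and merges them into higher tiers.
; SwordSummon and SwordFire route by tag to macros maintaining per-tier arrays; full batches merge at their average player-relative position, spawning the next tier.
; Tier 3's merge completion is disconnected, so Tier 4 never spawns; older _2 macros remain unused.
; Input handles movement, jump, cooldown dodge, fire-all, pause and FPS display.
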(event Custom|Spawn%20swords
  (bind _returnvalue (Transformation|GetActorLocation))
  (bind _randomlocation (Variables|Default|GetRandomLocation))
  (bind _returnvalue_2 (+ _returnvalue _randomlocation))
  ;[0 0 0] Spawn Swords
  (CallFunction|GetRandomLocation -2e+02 2e+02 1.5e+02 2.5e+02)
  (Game|SpawnActorfromClass "/Game/Actors/Swords/BP_Tier0Sword.BP_Tier0Sword_C" (Math|Transform|MakeTransform (Math|Vector|MakeVector 0.0 (.y _returnvalue_2) (.z _returnvalue_2)) "0, 0, 0" "1.000000,1.000000,1.000000") "AlwaysSpawn" "MultiplyWithRoot" 0 0))

(event Custom|ResumePlay
  (bind _returnvalue (Game|GetPlayerController 0))
  ;[0 0 0] IA PauseMenu
  (Variables|Default|SetIsRunning true)
  (Widget|RemovefromParent (Variables|Default|GetPauseMenuWidget))
  (Input|SetInputModeGameOnly _returnvalue false)
  (Variables|/Script/Engine.PlayerController|SetbShowMouseCursor _returnvalue false)
  (Game|SetGamePaused false))

(event Custom|CustomSpawn
  ;[0 0 0] Event Begin Play
  (CallFunction|SpawnSwords))

(event Custom|SwordFire
  (params (Fired%20Sword :type BP%20Base%20Flying%20Sword%20Object%20Reference%20%28by%20ref%29) (Tag :type Name))
  ;[0 0 0] SwordFire
  (Variables|Default|SetFired%20Sword Fired%20Sword)
  (switch name Tag
    (:Tier%200
      (|RemoveTier0_3))
    (:Tier%201
      (|RemoveTier1_3))
    (:Tier%202
      (|RemoveTier2_3))
    (:Tier%203
      (|RemoveTier3_3))))

(event Custom|SwordSummon
  (params (SummonedSword :type BP%20Base%20Flying%20Sword%20Object%20Reference%20%28by%20ref%29) (Tag :type Name))
  (Variables|Default|SetSummoned%20Sword SummonedSword)
  (switch name Tag
    (:Tier%200
      (|Tier0Merge_3))
    (:Tier%201
      (|Tier1Merge_3))
    (:Tier%202
      (|Tier2Merge_3))
    (:Tier%203
      (|Tier3Merge_3))))

(event Input|EnhancedActionEvents|EnhancedInputActionIA_KeyboardLR
  (params (ActionValue :type Vector%202D%20Structure) (ElapsedSeconds :type Float%20%28double-precision%29) (TriggeredSeconds :type Float%20%28double-precision%29) (InputAction :type Input%20Action%20Object%20Reference :default "/Game/Inputs/Actions/IA_KeyboardLR.IA_KeyboardLR"))
  ;[0 0 0] IA Keyboard Left/Right
  (Pawn|Input|AddMovementInput (Math|Vector|RotateVector (Math|Conversions|ToVector(Vector2D) ActionValue) (Transformation|GetActorRotation)) 1.0 false))

(event Input|EnhancedActionEvents|EnhancedInputActionIA_Jump
  (params (ActionValue :type Boolean) (ElapsedSeconds :type Float%20%28double-precision%29) (TriggeredSeconds :type Float%20%28double-precision%29) (InputAction :type Input%20Action%20Object%20Reference :default "/Game/Inputs/Actions/IA_Jump.IA_Jump"))
  ;[0 0 0] IA Jump
  (:Started
    (Character|Jump))
  (:Completed
    (Character|StopJumping)))

(event Input|EnhancedActionEvents|EnhancedInputActionIA_Dodge
  (params (ActionValue :type Boolean) (ElapsedSeconds :type Float%20%28double-precision%29) (TriggeredSeconds :type Float%20%28double-precision%29) (InputAction :type Input%20Action%20Object%20Reference :default "/Game/Inputs/Actions/IA_Dodge.IA_Dodge"))
  (bind _dodgeduration (Variables|Default|GetDodgeDuration))
  (bind _charactermovement (Variables|Character|GetCharacterMovement))
  ;[0 0 0] IA Dodge
  (if (Variables|Default|GetIsDodgeUp)
    (Variables|Default|SetIsDodgeUp false)
    (Variables|/Script/Engine.CharacterMovementComponent|SetMaxWalkSpeed _charactermovement (+ (Variables|/Script/Engine.CharacterMovementComponent|GetMaxWalkSpeed (Variables|Character|GetCharacterMovement)) 4e+03))
    (Utilities|FlowControl|Delay _dodgeduration)
    (Variables|/Script/Engine.CharacterMovementComponent|SetMaxWalkSpeed _charactermovement (- (Variables|/Script/Engine.CharacterMovementComponent|GetMaxWalkSpeed (Variables|Character|GetCharacterMovement)) 4e+03))
    (Utilities|FlowControl|Delay (- (Variables|Default|GetDodgeCooldown) _dodgeduration))
    (Variables|Default|SetIsDodgeUp true)
    (else
      (Development|PrintString "Dodge is on Cooldown" true true "(R=1.000000,G=0.000000,B=0.024480,A=1.000000)"))))

(event Input|EnhancedActionEvents|EnhancedInputActionIA_PauseMenu
  (params (ActionValue :type Boolean) (ElapsedSeconds :type Float%20%28double-precision%29) (TriggeredSeconds :type Float%20%28double-precision%29) (InputAction :type Input%20Action%20Object%20Reference :default "/Game/Inputs/Actions/IA_PauseMenu.IA_PauseMenu"))
  (bind _returnvalue (Game|GetPlayerController 0))
  ;[0 0 0] IA PauseMenu
  (if (Variables|Default|GetIsRunning)
    (Variables|Default|SetIsRunning false)
    (bind _returnvalue_2 (UserInterface|CreateWidget "/Game/UI/PauseMenu.PauseMenu_C" _returnvalue))
    (bind _output_get (Variables|Default|SetPauseMenuWidget _returnvalue_2))
    (UserInterface|Viewport|AddtoViewport _output_get 0)
    (Input|SetInputModeGameandUI _returnvalue _output_get "DoNotLock" true false)
    (Variables|/Script/Engine.PlayerController|SetbShowMouseCursor _returnvalue true)
    (Game|SetGamePaused true)
    (else
      (CallFunction|ResumePlay))))

(event Input|EnhancedActionEvents|EnhancedInputActionIA_FireAll
  (params (ActionValue :type Boolean) (ElapsedSeconds :type Float%20%28double-precision%29) (TriggeredSeconds :type Float%20%28double-precision%29) (InputAction :type Input%20Action%20Object%20Reference :default "/Game/Inputs/Actions/IA_FireAll.IA_FireAll"))
  ;[0 0 0] IA FireAll
  (Default|CallOnFIreAll)
  (Development|PrintString "Firing All!" true true "(R=1.000000,G=0.000000,B=0.799690,A=1.000000)"))

(event EventBeginPlay
  ;[0 0 0] Event Begin Play
  (CallFunction|EasyAddMappingContext "/Game/Inputs/IM_Playing.IM_Playing")
  (Utilities|Time|SetTimerbyEvent (delegate Custom|CustomSpawn) (/ 1.0 (Variables|Default|GetSwordsPerSecond)) true)
  (CallFunction|SpawnSwords))

(event Input|ActionEvents|InputActionShowFPS
  (params (Key :type Key%20Structure))
  (:Pressed
    (Development|ExecuteConsoleCommand "stat fps" (Game|GetPlayerController 0))))

(fn ConstructionScript)

(fn GetRandomLocation
  (params (Min%20Y :type Float%20%28double-precision%29) (Max%20Y :type Float%20%28double-precision%29) (Min%20Height :type Float%20%28double-precision%29) (Max%20Height :type Float%20%28double-precision%29))
  (Variables|Default|SetRandomLocation (Math|Vector|MakeVector 0.0 (Math|Random|RandomFloatinRange Min%20Y Max%20Y) (Math|Random|RandomFloatinRange Min%20Height Max%20Height))))