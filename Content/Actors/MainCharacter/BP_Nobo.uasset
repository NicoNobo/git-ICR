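; BP_Nobo is the player character, handling left/right movement with mesh lean, jump, a cooldown-gated speed-boost dodge, pause menu and FPS display.
; DoOnce gates limit lean changes and jump repeats, and holding both directions halts movement.
; FireAll calls a dispatcher, while interface functions expose its orientation vectors and X position.
; Tiered sword merge and remove graphs are present but not called from the event graph, with Tier 0 merging partly disconnected.
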(event Custom|Reset%20Left
  ;[0 0 0] IA LEFT AND RIGHT + ROTATION BASED ON DIRECTION
  (Utilities|FlowControl|DoOnce false) ; enters at Reset
)

(event Custom|ResumePlay
  (bind _returnvalue (Game|GetPlayerController 0))
  ;[0 0 0] IA PauseMenu
  (Variables|Default|SetIsRunning true)
  (Widget|RemovefromParent (Variables|Default|GetPauseMenuWidget))
  (Input|SetInputModeGameOnly _returnvalue false)
  (Variables|/Script/Engine.PlayerController|SetbShowMouseCursor _returnvalue false)
  (Game|SetGamePaused false))

(event Custom|Reset%20Right
  ;[0 0 0] IA LEFT AND RIGHT + ROTATION BASED ON DIRECTION
  (Utilities|FlowControl|DoOnce false) ; enters at Reset
)

(event Custom|Reset%20Both
  ;[0 0 0] IA LEFT AND RIGHT + ROTATION BASED ON DIRECTION
  (Utilities|FlowControl|DoOnce false) ; enters at Reset
)

(event Input|EnhancedActionEvents|EnhancedInputActionIA_Jump
  (params (ActionValue :type Boolean) (ElapsedSeconds :type Float%20%28double-precision%29) (TriggeredSeconds :type Float%20%28double-precision%29) (InputAction :type Input%20Action%20Object%20Reference :default "/Game/Inputs/Actions/IA_Jump.IA_Jump"))
  ;[0 0 0] IA Jump
  (:Ongoing
    (Utilities|FlowControl|DoOnce false :!label _label
      (:Completed
        (Character|Jump)
        (Audio|PlaySound2D "/Game/Audio/Jump1.Jump1" 1.0 1.0 0.0 0 0)
        (Utilities|FlowControl|Delay 1.75)
        (goto _label Reset))))
  (:Completed
    (Character|StopJumping)))

(event Input|EnhancedActionEvents|EnhancedInputActionIA_KeyboardLeft
  (params (ActionValue :type Vector%202D%20Structure) (ElapsedSeconds :type Float%20%28double-precision%29) (TriggeredSeconds :type Float%20%28double-precision%29) (InputAction :type Input%20Action%20Object%20Reference :default "/Game/Inputs/Actions/IA_KeyboardLeft.IA_KeyboardLeft"))
  ;[0 0 0] IA LEFT AND RIGHT + ROTATION BASED ON DIRECTION
  (:Triggered
    (if (not (and (== (Variables|Default|GetLeftActive) true) (== (Variables|Default|GetRightActive) true)))
      (Pawn|Input|AddMovementInput (Math|Vector|RotateVector (Math|Conversions|ToVector(Vector2D) ActionValue) (Transformation|GetActorRotation)) 1.0 false)
      (Utilities|FlowControl|DoOnce false
        (:Completed
          (Transformation|SetRelativeRotation (Variables|Character|GetMesh) "-7.500000,-90.000000,10.000000" false false)
          (Variables|Default|SetLeftActive true)))
      (else
        (Utilities|FlowControl|DoOnce false
          (:Completed
            (Transformation|SetRelativeRotation (Variables|Character|GetMesh) "0.000000,-90.000000,10.000000" false false))))))
  (:Completed
    (Transformation|SetRelativeRotation (Variables|Character|GetMesh) "0.000000,-90.000000,10.000000" false false)
    (CallFunction|ResetLeft)
    (CallFunction|ResetRight)
    (CallFunction|ResetBoth)
    (Variables|Default|SetLeftActive false)))

(event Input|EnhancedActionEvents|EnhancedInputActionIA_Dodge
  (params (ActionValue :type Boolean) (ElapsedSeconds :type Float%20%28double-precision%29) (TriggeredSeconds :type Float%20%28double-precision%29) (InputAction :type Input%20Action%20Object%20Reference :default "/Game/Inputs/Actions/IA_Dodge.IA_Dodge"))
  (bind _dodgeduration (Variables|Default|GetDodgeDuration))
  (bind _charactermovement (Variables|Character|GetCharacterMovement))
  ;[0 0 0] IA Dodge
  (if (Variables|Default|GetIsDodgeUp)
    (Variables|Default|SetIsDodgeUp false)
    (Audio|PlaySound2D "/Game/Audio/Dash5.Dash5" 1.0 1.0 0.0 0 0)
    (Variables|/Script/Engine.CharacterMovementComponent|SetMaxWalkSpeed _charactermovement (+ (Variables|/Script/Engine.CharacterMovementComponent|GetMaxWalkSpeed (Variables|Character|GetCharacterMovement)) 4e+03))
    (Utilities|FlowControl|Delay _dodgeduration)
    (Variables|/Script/Engine.CharacterMovementComponent|SetMaxWalkSpeed _charactermovement (- (Variables|/Script/Engine.CharacterMovementComponent|GetMaxWalkSpeed (Variables|Character|GetCharacterMovement)) 4e+03))
    (Utilities|FlowControl|Delay (- (Variables|Default|GetDodgeCooldown) _dodgeduration))
    (Variables|Default|SetIsDodgeUp true)
    (else
      (Development|PrintString "Dodge is on Cooldown" true true "(R=1.000000,G=0.000000,B=0.024480,A=1.000000)"))))

(event Input|EnhancedActionEvents|EnhancedInputActionIA_PauseMenu
  (params (ActionValue :type Boolean) (ElapsedSeconds :type Float%20%28double-precision%29) (TriggeredSeconds :type Float%20%28double-precision%29) (InputAction :type Input%20Action%20Object%20Reference :default "/Game/Inputs/Actions/IA_PauseMenu.IA_PauseMenu"))
  (bind _returnvalue (Game|GetPlayerController 0))
  ;[0 0 0] IA PauseMenu
  (if (Variables|Default|GetIsRunning)
    (Variables|Default|SetIsRunning false)
    (bind _returnvalue_2 (UserInterface|CreateWidget "/Game/UI/PauseMenu.PauseMenu_C" _returnvalue))
    (bind _output_get (Variables|Default|SetPauseMenuWidget _returnvalue_2))
    (UserInterface|Viewport|AddtoViewport _output_get 0)
    (Input|SetInputModeGameandUI _returnvalue _output_get "DoNotLock" true false)
    (Variables|/Script/Engine.PlayerController|SetbShowMouseCursor _returnvalue true)
    (Game|SetGamePaused true)
    (else
      (CallFunction|ResumePlay))))

(event Input|EnhancedActionEvents|EnhancedInputActionIA_FireAll
  (params (ActionValue :type Boolean) (ElapsedSeconds :type Float%20%28double-precision%29) (TriggeredSeconds :type Float%20%28double-precision%29) (InputAction :type Input%20Action%20Object%20Reference :default "/Game/Inputs/Actions/IA_FireAll.IA_FireAll"))
  ;[0 0 0] IA FireAll
  (Default|CallOnFIreAll)
  (Development|PrintString "Firing All!" true true "(R=1.000000,G=0.000000,B=0.799690,A=1.000000)"))

(event Input|EnhancedActionEvents|EnhancedInputActionIA_KeyboardRight
  (params (ActionValue :type Vector%202D%20Structure) (ElapsedSeconds :type Float%20%28double-precision%29) (TriggeredSeconds :type Float%20%28double-precision%29) (InputAction :type Input%20Action%20Object%20Reference :default "/Game/Inputs/Actions/IA_KeyboardRight.IA_KeyboardRight"))
  ;[0 0 0] IA LEFT AND RIGHT + ROTATION BASED ON DIRECTION
  (:Triggered
    (if (not (and (== (Variables|Default|GetLeftActive) true) (== (Variables|Default|GetRightActive) true)))
      (Pawn|Input|AddMovementInput (Math|Vector|RotateVector (Math|Conversions|ToVector(Vector2D) ActionValue) (Transformation|GetActorRotation)) 1.0 false)
      (Utilities|FlowControl|DoOnce false
        (:Completed
          (Transformation|SetRelativeRotation (Variables|Character|GetMesh) "7.500000,-90.000000,10.000000" false false)
          (Variables|Default|SetRightActive true)))
      (else
        (Utilities|FlowControl|DoOnce false
          (:Completed
            (Transformation|SetRelativeRotation (Variables|Character|GetMesh) "0.000000,-90.000000,10.000000" false false))))))
  (:Completed
    (Transformation|SetRelativeRotation (Variables|Character|GetMesh) "0.000000,-90.000000,10.000000" false false)
    (CallFunction|ResetRight)
    (CallFunction|ResetLeft)
    (CallFunction|ResetBoth)
    (Variables|Default|SetRightActive false)))

(event EventBeginPlay
  ;[0 0 0] Event Begin Play
  (bind _returnvalue (Actor|GetActorOfClass "/Game/Actors/SwordManager.SwordManager_C"))
  (Variables|Default|SetSword%20Manager _returnvalue)
  (CallFunction|EasyAddMappingContext "/Game/Inputs/IM_Playing.IM_Playing")
  (Audio|PlaySound2D "/Game/Audio/Song2.Song2" 1.0 1.0 0.0 0 0))

(event Input|ActionEvents|InputActionShowFPS
  (params (Key :type Key%20Structure :default "None"))
  ;[1 1 1] On TAB SHOW FPS
  (:Pressed
    (Development|ExecuteConsoleCommand "stat fps" (Game|GetPlayerController 0))))

(fn ConstructionScript)

(fn IFGetVectors
  (bind _returnvalue (Transformation|GetActorRotation))
  (return (Math|Vector|GetUpVector _returnvalue) (Math|Vector|GetRightVector _returnvalue)))

(fn IFGetX
  (return (.x (Transformation|GetActorLocation))))