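; BP_ForestPlane is a child Blueprint that defines forest decoration for three zones as instanced meshes.
; Each zone has an Array event registering its meshes and a Decorate event calling AddInstance with a scale range and full random rotation.
; Zone 1 mixes three meshes, using a random switch weighted toward Mesh3, while Zones 2 and 3 each place a single mesh.
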(event EventZone3Decorate
  ;[0 0 0] Zone 3
  (switch int 0
    (:0
      (CallFunction|AddInstance (Variables|Default|GetMesh1) 0.35 0.55 3.6e+02))))

(event EventZone1Array
  ;[0 0 0] Zone 1
  (Utilities|Array|Add (Variables|Default|GetInstances) (Variables|Default|GetMesh1))
  (Utilities|Array|Add (Variables|Default|GetInstances) (Variables|Default|GetMesh2))
  (Utilities|Array|Add (Variables|Default|GetInstances) (Variables|Default|GetMesh3)))

(event EventZone1Decorate
  ;[0 0 0] Zone 1
  (switch int (Math|Random|RandomIntegerinRange 0 5)
    (:0
      (CallFunction|AddInstance (Variables|Default|GetMesh1) 0.35 0.55 3.6e+02))
    (:1
      (CallFunction|AddInstance (Variables|Default|GetMesh2) 0.4 0.7 3.6e+02))
    (:2
      (CallFunction|AddInstance (Variables|Default|GetMesh3) 2.0 5.0 3.6e+02 :!label _label))
    (:3
      (goto _label))
    (:4
      (goto _label))
    (:5
      (goto _label))))

(event EventZone2Array
  ;[0 0 0] Zone 2
  (Utilities|Array|Add (Variables|Default|GetInstances) (Variables|Default|GetMesh3)))

(event EventZone2Decorate
  ;[0 0 0] Zone 2
  (switch int 0
    (:0
      (CallFunction|AddInstance (Variables|Default|GetMesh3) 2.0 5.0 3.6e+02))))

(event EventZone3Array
  ;[0 0 0] Zone 3
  (Utilities|Array|Add (Variables|Default|GetInstances) (Variables|Default|GetMesh1)))

(fn ConstructionScript
  (|CallParentFunction))