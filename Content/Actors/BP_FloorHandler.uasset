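; BP_FloorHandler is a trigger actor that recycles scrolling floor tiles to keep a continuous floor.
; When an actor overlaps its Box, it spawns a new BP_ScrollingFloor ahead along X, offset from that actor by tile spacing times tile count, then destroys the overlapping actor.
; The overlapping actor's class is not checked, the offset is hard-coded, and each spawn location is printed for debugging.
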(event OnComponentBeginOverlap(Box)
  (params (OverlappedComponent :type Primitive%20Component%20Object%20Reference) (OtherActor :type Actor%20Object%20Reference) (OtherComp :type Primitive%20Component%20Object%20Reference) (OtherBodyIndex :type Integer) (bFromSweep :type Boolean) (SweepResult :type Hit%20Result%20Structure%20%28by%20ref%29))
  (bind _output_get (Variables|Default|SetOther%20Actor OtherActor))
  (Variables|Default|SetNewSpawnLocation (Math|Vector|MakeVector (+ (* 6e+03 4.0) (.x (Transformation|GetActorLocation _output_get))) (.y (Transformation|GetActorLocation _output_get)) (.z (Transformation|GetActorLocation _output_get))))
  (Game|SpawnActorfromClass "/Game/Actors/BP_ScrollingFloor.BP_ScrollingFloor_C" (Math|Transform|MakeTransform (Variables|Default|GetNewSpawnLocation) "0, 0, 0" "1.000000,1.000000,1.000000") "AdjustIfPossibleButAlwaysSpawn" "MultiplyWithRoot" 0 0)
  (Development|PrintString (Utilities|String|Append "Spawning New Floor at location:" (Utilities|String|ToString(Vector) (Variables|Default|GetNewSpawnLocation))))
  (Actor|DestroyActor (Variables|Default|GetOther%20Actor)))

(fn ConstructionScript)