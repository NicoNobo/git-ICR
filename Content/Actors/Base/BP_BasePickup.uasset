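; BP_BasePickup is a base pickup actor that BP_Nobo characters collect by overlapping its hitbox.
; An overlap calls OnPlayerOverlap, which checks CanBePickedUp (true by default) before OnPickup plays an optional sound and destroys the actor.
; The construction script creates a dynamic collectible material tinted by the Color variable.
; A separate NoTeleport event also destroys the pickup, without sound.
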(event OnComponentBeginOverlap(Hitbox)
  (params (OverlappedComponent :type Primitive%20Component%20Object%20Reference) (OtherActor :type Actor%20Object%20Reference) (OtherComp :type Primitive%20Component%20Object%20Reference) (OtherBodyIndex :type Integer) (bFromSweep :type Boolean) (SweepResult :type Hit%20Result%20Structure%20%28by%20ref%29))
  (bind _asbp_nobo (Utilities|Casting|CastToBP_Nobo OtherActor))
  (CallFunction|OnPlayerOverlap _asbp_nobo))

(event Custom|OnPlayerOverlap
  (params (Character :type BP%20Nobo%20Object%20Reference))
  (bind _canbepickedup (CallFunction|CanbePickedUp))
  (if _canbepickedup
    (CallFunction|OnPickup Character)))

(event Custom|OnPickup
  (params (Character :type BP%20Nobo%20Object%20Reference))
  (bind _pickupsound (Variables|Default|GetPickupSound)
    (:then
      (Audio|PlaySoundatLocation _pickupsound (Transformation|GetWorldLocation (Variables|Default|GetStaticMesh)) "0, 0, 0" 1.0 1.0 0.0 0 0 0 0))
    (:else
      _))
  (Actor|DestroyActor))

(event EventBeginPlay
  (|CallParentFunction) ; This node is disabled and will not be called.\nDrag off pins to build functionality.
)

(event Collision|EventActorBeginOverlap
  (params (OtherActor :type Actor%20Object%20Reference)))

(event EventTick
  (params (DeltaSeconds :type Float%20%28single-precision%29))
  (|CallParentFunction DeltaSeconds) ; This node is disabled and will not be called.\nDrag off pins to build functionality.
)

(event EventNoTeleport
  (Actor|DestroyActor))

(fn ConstructionScript
  (|CallParentFunction)
  (bind _returnvalue (Rendering|Material|CreateDynamicMaterialInstance (Variables|Default|GetStaticMesh) 0 "/Game/Assets/MI_CollectibleMaterial.MI_CollectibleMaterial" "None" :!class /Script/Engine.PrimitiveComponent))
  (bind _output_get (Variables|Default|SetMaterial _returnvalue))
  (Rendering|Material|SetVectorParameterValue _output_get "Color" (Variables|Default|GetColor) :!class /Script/Engine.MaterialInstanceDynamic))

(fn CanbePickedUp
  (return true))