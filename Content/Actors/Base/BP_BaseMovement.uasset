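; BP_BaseMovement is a base actor that moves at the map speed and loops back along X.
; It caches the map speed on BeginPlay and refreshes it whenever GI_ICR fires OnMapSpeedChange.
; Tick computes the new location from that speed; once X reaches TeleportX, it shifts by SpawnX minus TeleportX, preserving the overshoot.
; An empty AfterTeleport event follows each wrap as a hook.
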(event Custom|AfterTeleport)

(event Custom|Update%20Map%20Speed
  ;[0 0 0] Event Begin Play / UpdateMapSpeed and Bind to OnMapSpeedChange
  (bind _mapspeed (CallFunction|GetMapSpeed))
  (Variables|Default|SetMapSpeed _mapspeed))

(event EventTick
  (params (DeltaSeconds :type Float%20%28single-precision%29))
  ;[0 0 0] Event Tick / Movement / IF Teleport Back
  (bind _new_location (CallFunction|GetNewLocation DeltaSeconds (Variables|Default|GetMapSpeed) (Transformation|GetActorLocation)))
  (Variables|Default|SetNew%20Location _new_location)
  (if (not (<= (.x (Variables|Default|GetNew%20Location)) (Variables|Default|GetTeleportX)))
    (Transformation|SetActorLocation (Variables|Default|GetNew%20Location) false false)
    (else
      (Transformation|SetActorLocation (Math|Vector|MakeVector (+ (.x (Variables|Default|GetNew%20Location)) (- (Variables|Default|GetSpawnX) (Variables|Default|GetTeleportX))) (.y (Variables|Default|GetNew%20Location)) (.z (Variables|Default|GetNew%20Location))) false false)
      (CallFunction|AfterTeleport))))

(event EventBeginPlay
  ;[0 0 0] Event Begin Play / UpdateMapSpeed and Bind to OnMapSpeedChange
  (CallFunction|UpdateMapSpeed)
  (bind _asgi_icr (Utilities|Casting|CastToGI_ICR (Game|GetGameInstance)))
  (EventDispatchers|AssignOnMapSpeedChange _asgi_icr (delegate Custom|Update%20Map%20Speed)))

(fn ConstructionScript)