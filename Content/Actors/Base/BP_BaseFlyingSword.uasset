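; Base flying sword that hovers around the BP_Nobo character with randomized sine bobbing, then launches as a projectile.
; After a hold time or the character's fire-all event, a timeline pulls it in front of the character before launch.
; It sticks on hit and scrolls with the GI_ICR map speed, or despawns at a distance if airborne.
; It reports spawning, firing and merging to SwordManager; merging lerps it to an offset and destroys it.
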(event OnComponentHit(Hitbox)
  (params (HitComponent :type Primitive%20Component%20Object%20Reference) (OtherActor :type Actor%20Object%20Reference) (OtherComp :type Primitive%20Component%20Object%20Reference) (NormalImpulse :type Vector :default "0, 0, 0") (Hit :type Hit%20Result%20Structure%20%28by%20ref%29))
  ;[0 0 0] On Component Hit
  (Variables|Default|SetIsStuck true)
  (Game|Components|ProjectileMovement|SetVelocityinLocalSpace (Variables|Default|GetProjectileMovement) "0, 0, 0"))

(event Custom|FireSequence
  (bind _character (Variables|Default|GetCharacter))
  (bind _returnvalue (Transformation|GetActorLocation _character))
  ;[0 0 0] FireSequence
  (if (not (Variables|Default|GetIsMerging))
    (if (not (Variables|Default|GetHasBeenFired))
      (Variables|Default|SetIsHolding false)
      (Variables|Default|SetHasBeenFired true)
      (Default|SwordFired (Variables|Default|GetSword%20Manager) self (Utilities|Array|Get(acopy) (Variables|Actor|GetTags)))
      (bind _alpha (Timeline|SwordToCenter PlayFromStart)
        (:Update
          (Transformation|SetActorRelativeLocation (Math|Vector|Lerp(Vector) (Transformation|GetActorLocation) (Math|Vector|MakeVector (+ (.x _returnvalue) 1.5e+02) (+ (.y _returnvalue) (Variables|Default|GetShootingY)) (+ (.z _returnvalue) (Variables|Default|GetShootingZ))) _alpha)))
        (:Finished
          (Transformation|SetActorRotation (Math|Rotator|MakeRotator (Math|Random|RandomFloatinRange -3.6e+02 3.6e+02) 0.0 0.0))
          (Game|Components|ProjectileMovement|SetVelocityinLocalSpace (Variables|Default|GetProjectileMovement) "2000.000000,0.000000,0.000000"))))))

(event Custom|HoldingMovement
  (bind _randomlocation (Variables|Default|GetRandomLocation))
  (bind _character (Variables|Default|GetCharacter))
  (bind _returnvalue (Transformation|GetActorLocation _character))
  (bind _returnvalue_2 (+ _returnvalue _randomlocation))
  ;[0 0 0] HoldingMovement
  (Transformation|SetActorLocation (Math|Vector|MakeVector 0.0 (+ (.y _returnvalue_2) (Variables|Default|GetBobbingY)) (+ (.z _returnvalue_2) (Variables|Default|GetBobbingZ))) false false))

(event Custom|EarlyFire
  ;[0 0 0] Event Begin Play
  (CallFunction|FireSequence))

(event Custom|BobbingCalculator
  ;[0 0 0] BobbingCalculator
  (Variables|Default|SetBobValue (* (Variables|Default|GetBobbingDistance) (Math|Trig|Sin(Degrees) (* (Actor|GetGameTimeSinceCreation) (Variables|Default|GetBobbingSpeed)))))
  (if (Variables|Default|GetBobBoolY)
    (Variables|Default|SetBobbingY (Variables|Default|GetBobValue))
    (else
      (Variables|Default|SetBobbingY (* (Variables|Default|GetBobValue) -1.0))))
  (if (Variables|Default|GetBobBoolZ)
    (Variables|Default|SetBobbingZ (Variables|Default|GetBobValue))
    (else
      (Variables|Default|SetBobbingZ (* (Variables|Default|GetBobValue) -1.0)))))

(event Custom|FollowTarget
  (params (DeltaSeconds :type Float%20%28double-precision%29))
  (bind _returnvalue (Transformation|GetActorLocation))
  ;[0 0 0] Follow Target
  (Transformation|SetActorRelativeLocation (Math|Vector|MakeVector (- (.x _returnvalue) (* DeltaSeconds (Variables|Default|GetMapSpeed))) (.y _returnvalue) (.z _returnvalue))))

(event Custom|Merge
  (params (MergeOffset :type Vector))
  ;[0 0 0] Merge
  (Variables|Default|SetIsMerging true)
  (Actor|Tick|SetActorTickEnabled false)
  (bind _alpha (Timeline|Timeline Play)
    (:Update
      (Transformation|SetActorRelativeLocation (Math|Vector|Lerp(Vector) (Transformation|GetActorLocation) (+ MergeOffset (Transformation|GetActorLocation (Variables|Default|GetCharacter))) _alpha)))
    (:Finished
      (Default|FinishedMerging (Variables|Default|GetSword%20Manager) (Utilities|Array|Get(acopy) (Variables|Actor|GetTags)))
      (Actor|DestroyActor))))

(event Custom|Update%20Map%20Speed
  ;[0 0 0] Event Begin Play
  (bind _mapspeed (CallFunction|GetMapSpeed))
  (Variables|Default|SetMapSpeed _mapspeed))

(event EventBeginPlay
  ;[0 0 0] Event Begin Play
  (Transformation|SetActorRotation (Math|Rotator|MakeRotator (Math|Random|RandomFloatinRange -25.0 25.0) 0.0 0.0))
  (bind _asgi_icr (Utilities|Casting|CastToGI_ICR (Game|GetGameInstance)))
  (CallFunction|UpdateMapSpeed)
  (EventDispatchers|AssignOnMapSpeedChange _asgi_icr (delegate Custom|Update%20Map%20Speed))
  (EventDispatchers|BindEventtoOnFireAll (Variables|Default|GetCharacter) (delegate Custom|EarlyFire))
  (CallFunction|BobbingCalculator)
  (CallFunction|HoldingMovement)
  (Default|SwordSpawned (Variables|Default|GetSword%20Manager) self (Utilities|Array|Get(acopy) (Variables|Actor|GetTags)))
  (Utilities|FlowControl|Delay (Variables|Default|GetHoldingTime))
  (Variables|Default|SetIsHolding false)
  (if (not (Variables|Default|GetHasBeenFired))
    (CallFunction|FireSequence)))

(event EventTick
  (params (DeltaSeconds :type Float%20%28single-precision%29))
  ;[0 0 0] Event Tick
  (if (not (Variables|Default|GetIsStuck))
    (if (Variables|Default|GetIsHolding)
      (CallFunction|BobbingCalculator)
      (CallFunction|HoldingMovement)
      (elif (>= (.x (Transformation|GetActorLocation)) 1.5e+04)
        (Actor|DestroyActor)))
    (else
      (CallFunction|FollowTarget DeltaSeconds))))

(fn ConstructionScript
  (bind _returnvalue (Rendering|Material|CreateDynamicMaterialInstance (Variables|Default|GetStaticMesh) 0 "/Game/Lily/sworfd/MI_Blade.MI_Blade" "None" :!class /Script/Engine.PrimitiveComponent))
  (Rendering|Material|SetVectorParameterValue _returnvalue "Color" (Variables|Default|GetColor) :!class /Script/Engine.MaterialInstanceDynamic)
  (bind _returnvalue_2 (Actor|GetActorOfClass "/Game/Actors/MainCharacter/BP_Nobo.BP_Nobo_C"))
  (Variables|Default|SetCharacter _returnvalue_2)
  (bind _returnvalue_3 (Actor|GetActorOfClass "/Game/Actors/SwordManager.SwordManager_C"))
  (Variables|Default|SetSword%20Manager _returnvalue_3)
  (CallFunction|GetRandoms 1e+02 2e+02 5.0 1e+01 -2e+01 2e+01 -2e+01 2e+01))

(fn GetRandoms
  (params (MinBobSpeed :type Float%20%28double-precision%29) (MaxBobSpeed :type Float%20%28double-precision%29) (MinBobDistance :type Float%20%28double-precision%29) (MaxBobDistance :type Float%20%28double-precision%29) (MinShootingY :type Float%20%28double-precision%29) (MaxShootingY :type Float%20%28double-precision%29) (MinShootingHeight :type Float%20%28double-precision%29) (MaxShootingHeight :type Float%20%28double-precision%29))
  (Variables|Default|SetBobbingDistance (Math|Random|RandomFloatinRange MinBobDistance MaxBobDistance))
  (Variables|Default|SetBobbingSpeed (Math|Random|RandomFloatinRange MinBobSpeed MaxBobSpeed))
  (Variables|Default|SetRandomLocation (- (Transformation|GetActorLocation) (Transformation|GetActorLocation (Variables|Default|GetCharacter))))
  (Variables|Default|SetShootingRotation (Math|Random|RandomIntegerinRange -360 360))
  (Variables|Default|SetBobBoolY (Math|Random|RandomBool))
  (Variables|Default|SetBobBoolZ (Math|Random|RandomBool))
  (Variables|Default|SetShootingY (Math|Random|RandomFloatinRange MinShootingY MaxShootingY))
  (Variables|Default|SetShootingZ (Math|Random|RandomFloatinRange MinShootingHeight MaxShootingHeight)))