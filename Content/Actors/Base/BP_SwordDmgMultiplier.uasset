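; BP_SwordDmgMultiplier is a pickup that permanently or cumulatively raises the collecting character's sword damage multiplier.
; On pickup it converts MultiplierPercentToAdd to a fraction, adds it to the character's SwordDamageMultiplier, then runs the parent pickup logic.
; Its CanBePickedUp override calls the parent but always returns true, ignoring the parent's result.
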(event EventOnPickup
  (params (Character :type BP%20Obon%20Object%20Reference))
  (Variables|/Game/Actors/MainCharacter/BP_Obon.BP_Obon_C|SetSwordDamageMultiplier Character (+ (Variables|/Game/Actors/MainCharacter/BP_Obon.BP_Obon_C|GetSwordDamageMultiplier Character) (/ (Variables|Default|GetMultiplierPercentToAdd) 1e+02)))
  (|CallParentFunction Character))

(fn ConstructionScript
  (|CallParentFunction))

(fn CanbePickedUp
  (params (Character :type BP%20Obon%20Object%20Reference))
  (|CallParentFunction Character)
  (return true))