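; Base enemy actor that takes damage from flying swords and records kills or missed kills in the game instance.
; Sword hits on the cube hitbox store the sword, apply damage, and refresh the health bar and damage indicator widgets.
; At zero HP it increments Kills, while the NoTeleport event increments KillsMissed.
; Both paths destroy all stored swords along with the enemy.
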(event OnComponentHit(CubeHitbox)
  (params (HitComponent :type Primitive%20Component%20Object%20Reference) (OtherActor :type Actor%20Object%20Reference) (OtherComp :type Primitive%20Component%20Object%20Reference) (NormalImpulse :type Vector :default "0, 0, 0") (Hit :type Hit%20Result%20Structure%20%28by%20ref%29))
  ;[0 0 0] On Component Hit / Add sword to array / Reduce health / Update Healthbar / If Hp is below add a kill and destroy actors in array
  (bind _asbp_base_flying_sword (Utilities|Casting|CastToBP_BaseFlyingSword OtherActor)
    (:then
      (Utilities|Array|Add (Variables|Default|GetSwordArray) OtherActor)
      (bind (_damage _hp_afterdamage) (CallFunction|Damage (Variables|Default|GetCurrentHP) _asbp_base_flying_sword))
      (Variables|Default|SetDamage%20Number _damage)
      (Variables|Default|SetCurrentHP _hp_afterdamage)
      (CallFunction|UpdateHealthBar)
      (CallFunction|DamageText)
      (if (<= (Variables|Default|GetCurrentHP) 0.0)
        (CallFunction|OnDeath)))
    (:CastFailed
      (Development|PrintString "Casting Failed"))))

(event Custom|UpdateHealthBar
  ;[0 0 0] Update Healthbar
  (bind _aswb_health_bar (Utilities|Casting|CastToWB_HealthBar (UserInterface|GetWidget (Variables|Default|GetHealthBar))))
  (Progress|SetPercent (Variables|/Game/UI/WB_HealthBar.WB_HealthBar_C|GetHealthBar _aswb_health_bar) (/ (Variables|Default|GetCurrentHP) (Variables|Default|GetMaxHP))))

(event Custom|OnDeath
  ;[0 0 0] OnDeath
  (bind _asgi_icr (Utilities|Casting|CastToGI_ICR (Game|GetGameInstance)))
  (Math|Integer|IncrementInt (Variables|/Game/Blueprints/GI_ICR.GI_ICR_C|GetKills _asgi_icr)
    (:%20%20
      (Development|PrintString "Adding Kill" true true "(R=0.000000,G=0.065985,B=1.000000,A=1.000000)")
      (for _array_element (Variables|Default|GetSwordArray)
        (Actor|DestroyActor _array_element))
      (Actor|DestroyActor))))

(event Custom|DamageText
  ;[0 0 0] DamageText
  (bind _aswb_damage_indicator (Utilities|Casting|CastToWB_DamageIndicator (UserInterface|GetWidget (Variables|Default|GetDamageIndicator))))
  (Default|ApplyDamage _aswb_damage_indicator (Utilities|Text|ToText(Float) (Variables|Default|GetDamage%20Number) "HalfToEven")))

(event EventBeginPlay
  ;[0 0 0] Event Begin Play / Set HP
  (Variables|Default|SetCurrentHP (Variables|Default|GetMaxHP))
  (CallFunction|UpdateHealthBar)
  (|CallParentFunction))

(event EventNoTeleport
  (bind _asgi_icr (Utilities|Casting|CastToGI_ICR (Game|GetGameInstance)))
  (Variables|/Game/Blueprints/GI_ICR.GI_ICR_C|SetKillsMissed _asgi_icr (+ (Variables|/Game/Blueprints/GI_ICR.GI_ICR_C|GetKillsMissed _asgi_icr) 1))
  (Development|PrintString "Adding Missed KIl" true true "(R=1.000000,G=0.000000,B=0.826232,A=1.000000)")
  (for _array_element (Variables|Default|GetSwordArray)
    (Actor|DestroyActor _array_element))
  (Actor|DestroyActor))

(fn ConstructionScript)