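; BP_FloorTile is a floor tile actor with event hooks for post-teleport and post-branch handling.
; AfterTeleport calls Scroll on the GI_ICR game instance, then prints the current zone from its ZoneInt as debug text.
; AfterBranch forwards location, spawn X, teleport X and target to AfterBranchTeleportBack.
; The construction script only calls its parent, and BeginPlay, overlap and Tick are disabled stubs.
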(event EventBeginPlay
  (|CallParentFunction) ; This node is disabled and will not be called.\nDrag off pins to build functionality.
)

(event Collision|EventActorBeginOverlap
  (params (OtherActor :type Actor%20Object%20Reference)))

(event EventTick
  (params (DeltaSeconds :type Float%20%28single-precision%29))
  (|CallParentFunction DeltaSeconds) ; This node is disabled and will not be called.\nDrag off pins to build functionality.
)

(event EventAfterTeleport
  (bind _asgi_icr (Utilities|Casting|CastToGI_ICR (Game|GetGameInstance)))
  (Default|Scroll+ _asgi_icr)
  (switch int (Variables|/Game/Blueprints/GI_ICR.GI_ICR_C|GetZoneInt _asgi_icr)
    (:0
      (Development|PrintString "Zone 1"))
    (:1
      (Development|PrintString "Zone 2"))
    (:2
      (Development|PrintString "Zone 3"))))

(event EventAfterBranch
  (params (New%20Location :type Vector :default "0, 0, 0") (SpawnX :type Float%20%28double-precision%29) (TeleportX :type Float%20%28double-precision%29) (Target :type BP%20Base%20Movement%20Object%20Reference))
  (CallFunction|AfterBranchTeleportBack New%20Location SpawnX TeleportX Target))

(fn ConstructionScript
  (|CallParentFunction))