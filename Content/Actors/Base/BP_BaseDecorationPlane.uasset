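; Base decoration plane that randomly scatters instanced meshes around itself to dress the current zone.
; Empty per-zone Array and Decorate events act as child hooks, selected by ZoneInt in a counted loop that picks random XY points at zero Z.
; AddInstance applies random yaw and per-axis scale at that point.
; It decorates on BeginPlay, binds to GI_ICR's zone change, and clears and rescatters instances after teleporting.
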(event Custom|InitiateDecorate
  ;[0 0 0] Decorate
  (if (Variables|Default|GetIsEnabled)
    (switch int (Variables|Default|GetZoneInt)
      (:0
        (CallFunction|Zone1Array))
      (:1
        (CallFunction|Zone2Array))
      (:2
        (CallFunction|Zone3Array)))
    (while (<= (Variables|Default|GetDecorationCounter) (Variables|Default|GetHowManyDecorations?))
      (Math|Integer|IncrementInt (Variables|Default|GetDecorationCounter)
        (:%20%20
          (CallFunction|GetLocation)
          (switch int (Variables|Default|GetZoneInt)
            (:0
              (CallFunction|Zone1Decorate))
            (:1
              (CallFunction|Zone2Decorate))
            (:2
              (CallFunction|Zone3Decorate))))))))

(event Custom|AddInstance
  (params (InstanceMesh :type Instanced%20Static%20Mesh%20Component%20Object%20Reference) (Min%20Scale :type Float%20%28double-precision%29) (Max%20Scale :type Float%20%28double-precision%29) (RandomRotationRange :type Float%20%28double-precision%29))
  (bind _returnvalue (Math|Random|RandomFloatinRange Min%20Scale Max%20Scale))
  ;[0 0 0] AddInstance
  (Components|InstancedStaticMesh|AddInstance InstanceMesh (Math|Transform|MakeTransform (Variables|Default|GetSpawnArea) (Math|Rotator|MakeRotator 0.0 0.0 (Math|Random|RandomFloatinRange (* RandomRotationRange -1.0) RandomRotationRange)) (Math|Vector|MakeVector _returnvalue _returnvalue _returnvalue)) true))

(event Custom|Zone%201%20Array
  ;[0 0 0] Decorate
)

(event Custom|Zone%202%20Array
  ;[0 0 0] Decorate
)

(event Custom|ZoneInt++
  ;[1 1 1] Begin Play
  (Math|Integer|IncrementInt (Variables|Default|GetZoneInt)))

(event Custom|Zone%201%20Decorate
  ;[0 0 0] Decorate
)

(event Custom|Zone%202%20Decorate
  ;[0 0 0] Decorate
)

(event Custom|Zone%203%20Decorate
  ;[0 0 0] Decorate
)

(event Custom|Zone%203%20Array
  ;[0 0 0] Decorate
)

(event EventBeginPlay
  ;[1 1 1] Begin Play
  (|CallParentFunction)
  (CallFunction|InitiateDecorate)
  (bind _asgi_icr (Utilities|Casting|CastToGI_ICR (Game|GetGameInstance)))
  (EventDispatchers|BindEventtoOnZoneChange _asgi_icr (delegate Custom|ZoneInt++)))

(event EventAfterTeleport
  ;[0 0 0] After  Teleport
  (if (Variables|Default|GetIsEnabled)
    (for _array_element (Variables|Default|GetInstances)
      (Components|InstancedStaticMesh|ClearInstances _array_element))
    (Utilities|Array|Clear (Variables|Default|GetInstances))
    (Variables|Default|SetDecorationCounter 1)
    (CallFunction|InitiateDecorate)))

(fn ConstructionScript)

(fn GetLocation
  (bind _returnvalue (Transformation|GetActorLocation))
  (bind _x_range (Variables|Default|GetX%20Range))
  (bind _y_range (Variables|Default|GetY%20Range))
  (Variables|Default|SetSpawnArea (Math|Vector|MakeVector (+ (.x _returnvalue) (Math|Random|RandomFloatinRange (Math|Conversions|ToFloat(Integer) (* _x_range -1)) (Math|Conversions|ToFloat(Integer) _x_range))) (+ (.y _returnvalue) (Math|Random|RandomFloatinRange (Math|Conversions|ToFloat(Integer) (* _y_range -1)) (Math|Conversions|ToFloat(Integer) _y_range))) 0.0)))