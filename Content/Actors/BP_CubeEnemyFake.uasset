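; BP_CubeEnemyFake is a cube enemy that starts at a fixed height and slides along negative X at the game instance's MapSpeed.
; Each hitbox hit stores the colliding actor in SwordArray, subtracts the player BP_Obon's sword base damage times multiplier, and updates health bar and damage indicator widgets.
; At zero health it adds a kill to GI_ICR, destroys every stored actor, then destroys itself.
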(event OnComponentHit(CubeHitbox)
  (params (HitComponent :type Primitive%20Component%20Object%20Reference) (OtherActor :type Actor%20Object%20Reference) (OtherComp :type Primitive%20Component%20Object%20Reference) (NormalImpulse :type Vector :default "0, 0, 0") (Hit :type Hit%20Result%20Structure%20%28by%20ref%29))
  ;[0 0 0] On Component Hit / Add sword to array / Reduce health / Update Healthbar / If Hp is below add a kill and destroy actors in array
  (Utilities|Array|AddUnique (Variables|Default|GetSwordArray) OtherActor)
  (bind _asbp_obon (Utilities|Casting|CastToBP_Obon (Game|GetPlayerCharacter 0)))
  (Variables|Default|SetDamageNumber (* (Variables|/Game/Actors/MainCharacter/BP_Obon.BP_Obon_C|GetSwordBaseDamage _asbp_obon) (Variables|/Game/Actors/MainCharacter/BP_Obon.BP_Obon_C|GetSwordDamageMultiplier _asbp_obon)))
  (Variables|Default|SetHealth (- (Variables|Default|GetHealth) (* (Variables|/Game/Actors/MainCharacter/BP_Obon.BP_Obon_C|GetSwordBaseDamage _asbp_obon) (Variables|/Game/Actors/MainCharacter/BP_Obon.BP_Obon_C|GetSwordDamageMultiplier _asbp_obon))))
  (CallFunction|UpdateHealthBar)
  (CallFunction|DamageText)
  (if (<= (Variables|Default|GetHealth) 0.0)
    (CallFunction|HealthBelowZero)))

(event Custom|UpdateHealthBar
  ;[0 0 0] Update Healthbar
  (bind _aswb_health_bar (Utilities|Casting|CastToWB_HealthBar (UserInterface|GetWidget (Variables|Default|GetHealthBar))))
  (Progress|SetPercent (Variables|/Game/UI/WB_HealthBar.WB_HealthBar_C|GetHealthBar _aswb_health_bar) (/ (Variables|Default|GetHealth) (Variables|Default|GetMaxHealth))))

(event Custom|HealthBelowZero
  ;[0 0 0] HealthBelowZero / What to do when enemy dies
  (bind _asgi_icr (Utilities|Casting|CastToGI_ICR (Game|GetGameInstance)))
  (Variables|/Game/Blueprints/GI_ICR.GI_ICR_C|SetKills _asgi_icr (+ (Variables|/Game/Blueprints/GI_ICR.GI_ICR_C|GetKills _asgi_icr) 1))
  (Development|PrintString "Adding Kill" true true "(R=0.000000,G=0.065985,B=1.000000,A=1.000000)")
  (for _array_element (Variables|Default|GetSwordArray)
    (Actor|DestroyActor _array_element))
  (Actor|DestroyActor))

(event Custom|DamageText
  ;[0 0 0] DamageText
  (bind _aswb_damage_indicator (Utilities|Casting|CastToWB_DamageIndicator (UserInterface|GetWidget (Variables|Default|GetDamageIndicator))))
  (Default|ApplyDamage _aswb_damage_indicator (Utilities|Text|ToText(Float) (Variables|Default|GetDamageNumber) "HalfToEven")))

(event EventBeginPlay
  (bind _returnvalue (Transformation|GetActorLocation))
  ;[0 0 0] Event Begin Play / Set location to floor / Grab some vars / Update Healthbar
  (Transformation|SetActorLocation (Math|Vector|MakeVector (.x _returnvalue) (.y _returnvalue) 1e+02) false false)
  (bind _asgi_icr (Utilities|Casting|CastToGI_ICR (Game|GetGameInstance)))
  (Variables|Default|SetMapSpeed (Variables|/Game/Blueprints/GI_ICR.GI_ICR_C|GetMapSpeed _asgi_icr))
  (Variables|Default|SetHealth (Variables|Default|GetMaxHealth))
  (CallFunction|UpdateHealthBar))

(event EventTick
  (params (DeltaSeconds :type Float%20%28single-precision%29))
  (bind _cubebody (Variables|Default|GetCubeBody))
  (bind _returnvalue (Transformation|GetWorldLocation _cubebody))
  ;[0 0 0] Event Tick / Move the cube
  (Transformation|SetActorLocation (Math|Vector|MakeVector (- (.x _returnvalue) (* DeltaSeconds (Variables|Default|GetMapSpeed))) (.y _returnvalue) (.z _returnvalue)) false false))

(fn ConstructionScript)