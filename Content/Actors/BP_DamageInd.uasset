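; BP_DamageInd is a short-lived damage number actor that shows a Damage value through its DmgInd widget.
; On BeginPlay it picks a smaller font when its X exceeds the player's interface-reported X by a large threshold, then passes damage and size to the widget.
; A Timeline lerps it to a randomized offset along the player-supplied up and right vectors, then destroys it.
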(event EventBeginPlay
  (bind _playerx (Class|BPIPlayer|IFGetX(Message) (Game|GetPlayerCharacter 0)))
  (if (>= (- (.x (Transformation|GetActorLocation)) _playerx) 55555.0)
    (Variables|Default|SetFont%20Size 40)
    (else
      (Variables|Default|SetFont%20Size 80)))
  (Class|BPIDamageInd|IFSetDamage(Message) (UserInterface|GetWidget (Variables|Default|GetDmgInd)) (Variables|Default|GetDamage) (Variables|Default|GetFont%20Size))
  (bind _output_get (Variables|Default|SetStartPos (Transformation|GetActorLocation)))
  (bind (_upvector _rightvector) (Class|BPIPlayer|IFGetVectors(Message) (Game|GetPlayerCharacter 0)))
  (Variables|Default|SetEndPos (+ _output_get (* _upvector (Math|Random|RandomFloatinRange 2e+02 2.5e+02)) (* _rightvector (Math|Random|RandomFloatinRange -8e+01 8e+01))))
  (bind _newtrack_0 (Timeline|Timeline Play)
    (:Update
      (Transformation|SetActorLocation (Math|Vector|Lerp(Vector) (Variables|Default|GetStartPos) (Variables|Default|GetEndPos) _newtrack_0) false false))
    (:Finished
      (Actor|DestroyActor))))

(fn ConstructionScript)