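; Flying sword projectile that hovers around BP_Obon, then launches forward.
; Tick bobs it at a randomized sine-driven offset until the holding delay or an early HoldingNoDelay call fires it once.
; Firing pauses Tick while a timeline lerps it in front of Obon, then sets projectile velocity.
; A hit re-enables Tick to scroll the stuck sword with GI_ICR's MapSpeed; timers destroy swords that never stick.
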(event OnComponentHit(DamageHitbox)
  (params (HitComponent :type Primitive%20Component%20Object%20Reference) (OtherActor :type Actor%20Object%20Reference) (OtherComp :type Primitive%20Component%20Object%20Reference) (NormalImpulse :type Vector :default "0, 0, 0") (Hit :type Hit%20Result%20Structure%20%28by%20ref%29))
  ;[0 0 0] On Component Hit
  (Variables|Default|SetIsStuck true)
  (Actor|Tick|SetActorTickEnabled true))

(event Custom|Destroy
  ;[0 0 0] Event Begin Play / Set timer for auto destroy / Get randoms / Actor Rotation / Holding / Grab Vars
  (if (not (Variables|Default|GetIsStuck))
    (Actor|DestroyActor)))

(event Custom|Holding
  ;[0 0 0] Holding Logic and Animation
  (Utilities|FlowControl|Delay (Variables|Default|GetHoldingTime))
  (if (not (Variables|Default|GetAlreadyFired))
    (Variables|Default|SetAlreadyFired true)
    (Actor|Tick|SetActorTickEnabled false)
    (bind _returnvalue (Actor|GetActorOfClass "/Game/Actors/MainCharacter/BP_Obon.BP_Obon_C"))
    (bind _alpha (Timeline|Sword Play)
      (:Update
        (Transformation|SetActorRelativeLocation (Math|Vector|Lerp(Vector) (Transformation|GetActorLocation) (Math|Vector|MakeVector (+ (.x (Transformation|GetActorLocation _returnvalue)) 1.5e+02) (+ (.y (Transformation|GetActorLocation _returnvalue)) (Variables|Default|GetRandomShootRangeLR)) (+ (.z (Transformation|GetActorLocation _returnvalue)) (Variables|Default|GetRandomShootRangeHeight))) _alpha)))
      (:Finished
        (Game|Components|ProjectileMovement|SetVelocityinLocalSpace (Variables|Default|GetProjectileMovement) "1200.000000,0.000000,0.000000")
        (Transformation|SetActorRotation (Math|Rotator|MakeRotator (Variables|Default|GetRandomXRotation) 0.0 0.0))))))

(event Custom|Holding%20No%20Delay
  ;[0 0 0] Holding Logic and Animation
  (if (not (Variables|Default|GetAlreadyFired))
    (Variables|Default|SetAlreadyFired true)
    (Utilities|Time|SetTimerbyEvent (delegate Custom|CustomEvent) 1e+01)
    (Actor|Tick|SetActorTickEnabled false)
    (bind _returnvalue (Actor|GetActorOfClass "/Game/Actors/MainCharacter/BP_Obon.BP_Obon_C"))
    (bind _alpha (Timeline|Sword Play)
      (:Update
        (Transformation|SetActorRelativeLocation (Math|Vector|Lerp(Vector) (Transformation|GetActorLocation) (Math|Vector|MakeVector (+ (.x (Transformation|GetActorLocation _returnvalue)) 1.5e+02) (+ (.y (Transformation|GetActorLocation _returnvalue)) (Variables|Default|GetRandomShootRangeLR)) (+ (.z (Transformation|GetActorLocation _returnvalue)) (Variables|Default|GetRandomShootRangeHeight))) _alpha)))
      (:Finished
        (Game|Components|ProjectileMovement|SetVelocityinLocalSpace (Variables|Default|GetProjectileMovement) "1200.000000,0.000000,0.000000")
        (Transformation|SetActorRotation (Math|Rotator|MakeRotator (Variables|Default|GetRandomXRotation) 0.0 0.0))))))

(event Custom|CustomEvent
  ;[0 0 0] Holding Logic and Animation
  (CallFunction|Destroy))

(event EventBeginPlay
  ;[0 0 0] Event Begin Play / Set timer for auto destroy / Get randoms / Actor Rotation / Holding / Grab Vars
  (Utilities|Time|SetTimerbyEvent (delegate Custom|Destroy) (+ 1e+01 (Variables|Default|GetHoldingTime)))
  (CallFunction|GetRandoms 100 200 5 10 6e+01 4e+01 0.0 2e+02 1.5e+02 2.5e+02)
  (Transformation|SetActorRotation (Math|Rotator|MakeRotator (Math|Random|RandomFloatinRange -2e+01 2e+01) 0.0 0.0))
  (CallFunction|Holding)
  (bind _asgi_icr (Utilities|Casting|CastToGI_ICR (Game|GetGameInstance)))
  (Variables|Default|SetMapSpeed (Variables|/Game/Blueprints/GI_ICR.GI_ICR_C|GetMapSpeed _asgi_icr)))

(event EventTick
  (params (DeltaSeconds :type Float%20%28single-precision%29))
  (bind _returnvalue (Transformation|GetActorLocation))
  (bind _returnvalue_2 (Actor|GetGameTimeSinceCreation))
  (bind _bobbingspeed (Variables|Default|GetBobbingSpeed))
  (bind _bobbingdistance (Variables|Default|GetBobbingDistance))
  (bind _returnvalue_3 (* _returnvalue_2 _bobbingspeed))
  (bind _returnvalue_4 (Math|Trig|Sin(Degrees) _returnvalue_3))
  (bind _returnvalue_5 (* _bobbingdistance _returnvalue_4))
  ;[0 0 0] Event Tick / Gives the swords a random X/Y/Z bobbing movement
  (if (not (Variables|Default|GetIsStuck))
    (bind _returnvalue_6 (Actor|GetActorOfClass "/Game/Actors/MainCharacter/BP_Obon.BP_Obon_C"))
    (if (Variables|Default|GetBoolY)
      (Variables|Default|SetY _returnvalue_5)
      (else
        (Variables|Default|SetY (* _returnvalue_5 -1.0))))
    (if (Variables|Default|GetBoolZ)
      (Variables|Default|SetZ _returnvalue_5)
      (else
        (Variables|Default|SetZ (* _returnvalue_5 -1.0))))
    (Transformation|SetActorRelativeLocation (Math|Vector|MakeVector 0.0 (+ (+ (.y (.location (Transformation|GetActorTransform _returnvalue_6))) (Variables|Default|GetRandomY)) (Variables|Default|GetY)) (+ (+ (.z (.location (Transformation|GetActorTransform _returnvalue_6))) (Variables|Default|GetRandomZ)) (Variables|Default|GetZ))))
    (else
      ;[0 0 0] Follows Enemy Movement
      (Transformation|SetActorRelativeLocation (Math|Vector|MakeVector (- (.x _returnvalue) (* DeltaSeconds (Variables|Default|GetMapSpeed))) (.y _returnvalue) (.z _returnvalue))))))

(fn ConstructionScript)

(fn GetRandoms
  (params (MinBobbingSpeed :type Integer) (MaxBobbingSpeed :type Integer) (MinBobbingDistance :type Integer) (MaxBobbingDistance :type Integer) (RandomShootLR :type Float%20%28double-precision%29) (RandomShootHeight :type Float%20%28double-precision%29) (MinLR :type Float%20%28double-precision%29) (MaxLR :type Float%20%28double-precision%29) (MinHeight :type Float%20%28double-precision%29) (MaxHeight :type Float%20%28double-precision%29))
  (bind _returnvalue (/ RandomShootHeight 2.0))
  (bind _returnvalue_2 (/ RandomShootLR 2.0))
  (Variables|Default|SetBoolY (Math|Random|RandomBool))
  (Variables|Default|SetBoolZ (Math|Random|RandomBool))
  (Variables|Default|SetRandomXRotation (Math|Random|RandomFloatinRange -3.6e+02 3.6e+02)) ; Randon Shooting Rotation
  (Variables|Default|SetBobbingSpeed (Math|Random|RandomIntegerinRange MinBobbingSpeed MaxBobbingSpeed))
  (Variables|Default|SetBobbingDistance (Math|Random|RandomIntegerinRange MinBobbingDistance MaxBobbingDistance))
  (Variables|Default|SetRandomShootRangeLR (Math|Random|RandomFloatinRange (- 0.0 _returnvalue_2) (+ 0.0 _returnvalue_2))) ; If 100 it'll be between -50 and 50
  (Variables|Default|SetRandomShootRangeHeight (Math|Random|RandomFloatinRange (- 0.0 _returnvalue) (+ 0.0 _returnvalue)))
  (if (Variables|Default|GetBoolY)
    (Variables|Default|SetRandomY (Math|Random|RandomFloatinRange MinLR MaxLR))
    (else
      (Variables|Default|SetRandomY (Math|Random|RandomFloatinRange (* MaxLR -1.0) (* MinLR -1.0)))))
  (Variables|Default|SetRandomZ (Math|Random|RandomFloatinRange MinHeight MaxHeight)) ; Random height between Min and Max
)