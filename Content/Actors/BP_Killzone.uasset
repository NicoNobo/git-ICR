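; BP_Killzone is a trigger volume that destroys any actor that begins overlapping its Hitbox.
; When the actor is a BP_CubeEnemy, it first increments KillsMissed on the GI_ICR game instance, recording an enemy the player failed to kill.
; Other actors skip the counter and go straight to destruction, and both branches carry empty PrintString calls.
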(event OnComponentBeginOverlap(Hitbox)
  (params (OverlappedComponent :type Primitive%20Component%20Object%20Reference) (OtherActor :type Actor%20Object%20Reference) (OtherComp :type Primitive%20Component%20Object%20Reference) (OtherBodyIndex :type Integer) (bFromSweep :type Boolean) (SweepResult :type Hit%20Result%20Structure%20%28by%20ref%29))
  (bind _output_get (Variables|Default|SetOther%20Actor OtherActor))
  (Utilities|Casting|CastToBP_CubeEnemy _output_get
    (:then
      (Development|PrintString "")
      (bind _asgi_icr (Utilities|Casting|CastToGI_ICR (Game|GetGameInstance)))
      (Variables|/Game/Blueprints/GI_ICR.GI_ICR_C|SetKillsMissed _asgi_icr (+ (Variables|/Game/Blueprints/GI_ICR.GI_ICR_C|GetKillsMissed _asgi_icr) 1)))
    (:CastFailed
      (Development|PrintString "")))
  (Actor|DestroyActor (Variables|Default|GetOther%20Actor)))

(fn ConstructionScript)