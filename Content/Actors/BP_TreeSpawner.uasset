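; BP_TreeSpawner is an actor that scatters BP_Tree actors in two bands either side of Y zero, leaving the middle clear.
; Tick prefills the X range with one tree per frame for about 80 frames, then disables itself, regardless of IsEnabled.
; When IsEnabled, a looping timer keeps spawning trees at the far X end.
; Each spawn randomizes side, yaw and uniform scale, and is skipped if collisions cannot be resolved.
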(event Custom|SpawnTree
  (Variables|Default|SetRandomScale (Math|Random|RandomFloatinRange 0.5 0.7))
  (if (Math|Random|RandomBool)
    (Variables|Default|SetRandomY (Math|Random|RandomFloatinRange (Variables|Default|GetMin%20Range) (Variables|Default|GetMax%20Range)))
    (else
      (Variables|Default|SetRandomY (Math|Random|RandomFloatinRange (* -1.0 (Variables|Default|GetMax%20Range)) (* -1.0 (Variables|Default|GetMin%20Range))))))
  (Game|SpawnActorfromClass "/Game/Actors/BP_Tree.BP_Tree_C" (Math|Transform|MakeTransform (Math|Vector|MakeVector 1.4e+04 (Variables|Default|GetRandomY) 0.0) (Math|Rotator|MakeRotator 0.0 0.0 (Math|Random|RandomFloatinRange -3.6e+02 3.6e+02)) (Math|Vector|MakeVector (Variables|Default|GetRandomScale) (Variables|Default|GetRandomScale) (Variables|Default|GetRandomScale))) "AdjustIfPossibleButDontSpawnIfColliding" "MultiplyWithRoot" 0 0))

(event EventTick
  (params (DeltaSeconds :type Float%20%28single-precision%29))
  (Variables|Default|SetLoadingFirstTrees (+ (Variables|Default|GetLoadingFirstTrees) 1))
  (Variables|Default|SetRandomScale (Math|Random|RandomFloatinRange 0.5 0.7))
  (if (Math|Random|RandomBool)
    (Variables|Default|SetRandomY (Math|Random|RandomFloatinRange (Variables|Default|GetMin%20Range) (Variables|Default|GetMax%20Range)))
    (else
      (Variables|Default|SetRandomY (Math|Random|RandomFloatinRange (* -1.0 (Variables|Default|GetMax%20Range)) (* -1.0 (Variables|Default|GetMin%20Range))))))
  (Game|SpawnActorfromClass "/Game/Actors/BP_Tree.BP_Tree_C" (Math|Transform|MakeTransform (Math|Vector|MakeVector (Math|Random|RandomFloatinRange 0.0 1.4e+04) (Variables|Default|GetRandomY) 0.0) (Math|Rotator|MakeRotator 0.0 0.0 (Math|Random|RandomFloatinRange -3.6e+02 3.6e+02)) (Math|Vector|MakeVector (Variables|Default|GetRandomScale) (Variables|Default|GetRandomScale) (Variables|Default|GetRandomScale))) "AdjustIfPossibleButDontSpawnIfColliding" "MultiplyWithRoot" 0 0)
  (if (>= (Variables|Default|GetLoadingFirstTrees) 80)
    (Actor|Tick|SetActorTickEnabled false)))

(event EventBeginPlay
  (if (Variables|Default|GetIsEnabled)
    (CallFunction|SpawnTree)
    (Utilities|Time|SetTimerbyEvent (delegate Custom|SpawnTree) 0.3 true)))

(fn ConstructionScript)