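; BP_DecorationPlane is an actor that randomly scatters trees and plants around itself as ground decoration.
; When enabled, it adds instances to three instanced mesh components on BeginPlay, using random points within an X/Y range at world Z zero, random yaw and per-axis scale.
; The random pick favours plants over the two tree types.
; AfterTeleport clears all instances and scatters a fresh set around the actor's new location.
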(event Custom|Decorate
  ;[0 0 0] Decorate
  (if (Variables|Default|GetIsEnabled)
    (while (<= (Variables|Default|GetDecorationCounter) (Variables|Default|GetHowManyDecorations?))
      (Math|Integer|IncrementInt (Variables|Default|GetDecorationCounter)
        (:%20%20
          (CallFunction|GetLocation)
          (switch int (Math|Random|RandomIntegerinRange 0 5)
            (:0
              (CallFunction|AddInstance (Variables|Default|GetTree1) 0.4 0.6 3.6e+02))
            (:1
              (CallFunction|AddInstance (Variables|Default|GetTree2) 0.3 0.5 3.6e+02))
            (:2
              (CallFunction|AddInstance (Variables|Default|GetPlant) 2.0 1e+01 3.6e+02 :!label _label))
            (:3
              (goto _label))
            (:4
              (goto _label))
            (:5
              (goto _label))))))))

(event Custom|AddInstance
  (params (InstanceMesh :type Instanced%20Static%20Mesh%20Component%20Object%20Reference) (Min%20Scale :type Float%20%28double-precision%29) (Max%20Scale :type Float%20%28double-precision%29) (RandomRotationRange :type Float%20%28double-precision%29))
  (bind _returnvalue (Math|Random|RandomFloatinRange Min%20Scale Max%20Scale))
  ;[0 0 0] AddInstance
  (Components|InstancedStaticMesh|AddInstance InstanceMesh (Math|Transform|MakeTransform (Variables|Default|GetSpawnArea) (Math|Rotator|MakeRotator 0.0 0.0 (Math|Random|RandomFloatinRange (* RandomRotationRange -1.0) RandomRotationRange)) (Math|Vector|MakeVector _returnvalue _returnvalue _returnvalue)) true))

(event EventBeginPlay
  ;[1 1 1] Begin Play
  (|CallParentFunction)
  (CallFunction|Decorate)
  (Utilities|Array|Add (Variables|Default|GetInstances) (Variables|Default|GetTree1))
  (Utilities|Array|Add (Variables|Default|GetInstances) (Variables|Default|GetTree2))
  (Utilities|Array|Add (Variables|Default|GetInstances) (Variables|Default|GetPlant)))

(event EventAfterTeleport
  (if (Variables|Default|GetIsEnabled)
    (for _array_element (Variables|Default|GetInstances)
      (Components|InstancedStaticMesh|ClearInstances _array_element))
    (Variables|Default|SetDecorationCounter 1)
    (CallFunction|Decorate)))

(fn ConstructionScript)

(fn GetLocation
  (bind _returnvalue (Transformation|GetActorLocation))
  (bind _x_range (Variables|Default|GetX%20Range))
  (bind _y_range (Variables|Default|GetY%20Range))
  (Variables|Default|SetSpawnArea (Math|Vector|MakeVector (+ (.x _returnvalue) (Math|Random|RandomFloatinRange (Math|Conversions|ToFloat(Integer) (* _x_range -1)) (Math|Conversions|ToFloat(Integer) _x_range))) (+ (.y _returnvalue) (Math|Random|RandomFloatinRange (Math|Conversions|ToFloat(Integer) (* _y_range -1)) (Math|Conversions|ToFloat(Integer) _y_range))) 0.0)))