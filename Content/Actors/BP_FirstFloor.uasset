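; BP_FirstFloor is a floor actor that scrolls along negative X to move the level past a fixed point.
; On BeginPlay it reads MapSpeed from the GI_ICR game instance.
; Each tick it sets the actor location from the Floor component's world position, shifted by MapSpeed scaled by delta time.
; A Hitbox overlap only prints a debug message.
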(event OnComponentBeginOverlap(Hitbox)
  (params (OverlappedComponent :type Primitive%20Component%20Object%20Reference) (OtherActor :type Actor%20Object%20Reference) (OtherComp :type Primitive%20Component%20Object%20Reference) (OtherBodyIndex :type Integer) (bFromSweep :type Boolean) (SweepResult :type Hit%20Result%20Structure%20%28by%20ref%29))
  (Development|PrintString "Overlaping"))

(event EventTick
  (params (DeltaSeconds :type Float%20%28single-precision%29))
  (bind _floor (Variables|Default|GetFloor))
  (bind _returnvalue (Transformation|GetWorldLocation _floor))
  (Transformation|SetActorLocation (Math|Vector|MakeVector (- (.x _returnvalue) (* DeltaSeconds (Variables|Default|GetMap%20Speed))) (.y _returnvalue) (.z _returnvalue)) false false))

(event EventBeginPlay
  (bind _asgi_icr (Utilities|Casting|CastToGI_ICR (Game|GetGameInstance)))
  (Variables|Default|SetMap%20Speed (Variables|/Game/Blueprints/GI_ICR.GI_ICR_C|GetMapSpeed _asgi_icr)))

(fn ConstructionScript)