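; BP_ScrollingFloor is a floor actor that scrolls along X and loops to form a repeating track.
; It caches the map speed on BeginPlay and each Tick moves to a location computed from that speed and delta time.
; Past a negative X threshold, it jumps forward by a fixed offset, calls Scroll on the GI_ICR game instance, and prints debug messages for the teleport and current zone.
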(event EventTick
  (params (DeltaSeconds :type Float%20%28single-precision%29))
  (bind _new_location (CallFunction|GetNewLocation DeltaSeconds (Variables|Default|GetMap%20Speed) (Transformation|GetActorLocation)))
  (Variables|Default|SetNew%20Location _new_location)
  (if (not (<= (.x (Variables|Default|GetNew%20Location)) -4e+03))
    (Transformation|SetActorLocation (Variables|Default|GetNew%20Location) false false)
    (else
      (Transformation|SetActorLocation (Math|Vector|MakeVector (+ (.x (Variables|Default|GetNew%20Location)) 2.4e+04) (.y (Variables|Default|GetNew%20Location)) (.z (Variables|Default|GetNew%20Location))) false false)
      (Development|PrintString (Utilities|String|Append "X Teleport:" (Utilities|String|ToString(Float) (+ (.x (Variables|Default|GetNew%20Location)) 2.4e+04))) true true "(R=1.000000,G=0.805385,B=0.000000,A=1.000000)")
      (bind _asgi_icr (Utilities|Casting|CastToGI_ICR (Game|GetGameInstance)))
      (Default|Scroll+ _asgi_icr)
      (switch int (Variables|/Game/Blueprints/GI_ICR.GI_ICR_C|GetZoneInt _asgi_icr)
        (:0
          (Development|PrintString "Zone 1"))
        (:1
          (Development|PrintString "Zone 2"))
        (:2
          (Development|PrintString "Zone 3"))))))

(event EventBeginPlay
  (bind _mapspeed (CallFunction|GetMapSpeed))
  (Variables|Default|SetMap%20Speed _mapspeed))

(fn ConstructionScript)