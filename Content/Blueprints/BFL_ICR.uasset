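; BFL_ICR is a function library of shared helpers for world scrolling and sword damage.
; GetMapSpeed reads the GameInstance speed, and GetNewLocation uses a given speed to step a location along negative X per frame.
; AfterBranchTeleportBack shifts a target by the spawn-to-teleport X offset, apparently to recycle scrolled actors.
; Damage multiplies a flying sword's base damage by BP_Nobo's multiplier and returns it with remaining HP.
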(fn GetMapSpeed
  (bind _asgi_icr (Utilities|Casting|CastToGI_ICR (Game|GetGameInstance)))
  (return (Variables|/Game/Blueprints/GI_ICR.GI_ICR_C|GetMapSpeed _asgi_icr)))

(fn GetNewLocation
  (params (Delta%20Seconds :type Float%20%28double-precision%29) (MapSpeed :type Integer) (Actor%20Location :type Vector))
  (return (Math|Vector|MakeVector (- (.x Actor%20Location) (* Delta%20Seconds MapSpeed)) (.y Actor%20Location) (.z Actor%20Location))))

(fn Damage
  (params (CurrentHP :type Float%20%28double-precision%29) (Object :type BP%20Base%20Flying%20Sword%20Object%20Reference))
  (bind _asbp_nobo (Utilities|Casting|CastToBP_Nobo (Game|GetPlayerCharacter 0)))
  (bind _asbp_base_flying_sword (Utilities|Casting|CastToBP_BaseFlyingSword Object))
  (return (* (Variables|/Game/Actors/Base/BP_BaseFlyingSword.BP_BaseFlyingSword_C|GetBaseDamage _asbp_base_flying_sword) (Variables|/Game/Actors/MainCharacter/BP_Nobo.BP_Nobo_C|GetSwordDamageMultiplier _asbp_nobo)) (- CurrentHP (* (Variables|/Game/Actors/Base/BP_BaseFlyingSword.BP_BaseFlyingSword_C|GetBaseDamage _asbp_base_flying_sword) (Variables|/Game/Actors/MainCharacter/BP_Nobo.BP_Nobo_C|GetSwordDamageMultiplier _asbp_nobo)))))

(fn AfterBranchTeleportBack
  (params (NewLocation :type Vector) (SpawnX :type Float%20%28double-precision%29) (TeleportX :type Float%20%28double-precision%29) (Target :type Actor%20Object%20Reference))
  (Transformation|SetActorLocation Target (Math|Vector|MakeVector (+ (.x NewLocation) (- SpawnX TeleportX)) (.y NewLocation) (.z NewLocation)) false false))