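; Game instance that holds player progress for a sword-merging game, along with map speed and zone state.
; Loads from the SG_Save slot on Init and saves on Shutdown, covering sword level, kills, misses and upgrade settings; NewGame overwrites the slot with default data.
; SetMapSpeed fires a change dispatcher.
; Every twelfth scroll advances the zone, but the zone-change dispatcher call is unwired.
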(event Custom|Scroll+
  (Variables|Default|SetScrollCounter (+ (Variables|Default|GetScrollCounter) 1))
  (if (>= (Variables|Default|GetScrollCounter) 12)
    (Variables|Default|SetScrollCounter 0)
    (Variables|Default|SetZoneInt (+ (Variables|Default|GetZoneInt) 1))))

(event Custom|SetMapSpeed
  (params (NewMapSpeed :type Integer))
  (Variables|Default|SetMapSpeed NewMapSpeed)
  (Default|CallOnMapSpeedChange))

(event EventInit
  (CallFunction|LoadGame))

(event EventShutdown
  (CallFunction|SaveGame))

(fn SaveGame
  (bind _returnvalue (SaveGame|CreateSaveGameObject "/Game/Blueprints/SG_Save.SG_Save_C"))
  (Default|SaveData _returnvalue (Variables|Default|GetSwordLevel) (Variables|Default|GetKills) (Variables|Default|GetKillsMissed) (Variables|Default|GetAttackSpeedCap) (Variables|Default|GetHowManySwordsToMerge) (Variables|Default|GetAutoMerge))
  (SaveGame|SaveGametoSlot _returnvalue (Variables|Default|GetSaveSlot)))

(fn LoadGame
  (bind _returnvalue (SaveGame|LoadGamefromSlot (Variables|Default|GetSaveSlot)))
  (bind _assg_save (Utilities|Casting|CastToSG_Save _returnvalue))
  (Variables|Default|SetSwordLevel (Variables|/Game/Blueprints/SG_Save.SG_Save_C|GetsSwordLevel _assg_save))
  (Variables|Default|SetKills (Variables|/Game/Blueprints/SG_Save.SG_Save_C|GetsKills _assg_save))
  (Variables|Default|SetKillsMissed (Variables|/Game/Blueprints/SG_Save.SG_Save_C|GetsKillsMissed _assg_save))
  (Variables|Default|SetAttackSpeedCap (Variables|/Game/Blueprints/SG_Save.SG_Save_C|GetsAttackSpeedCap _assg_save))
  (Variables|Default|SetHowManySwordsToMerge (Variables|/Game/Blueprints/SG_Save.SG_Save_C|GetsHowManySwordsToMerge _assg_save))
  (Variables|Default|SetAutoMerge (Variables|/Game/Blueprints/SG_Save.SG_Save_C|GetsAutoMerge _assg_save))
  (Development|PrintString "Finished Loading"))

(fn NewGame
  (bind _returnvalue (SaveGame|CreateSaveGameObject "/Game/Blueprints/SG_Save.SG_Save_C"))
  (Default|SaveData _returnvalue 0 0 0 0 0 false)
  (SaveGame|SaveGametoSlot _returnvalue (Variables|Default|GetSaveSlot)))